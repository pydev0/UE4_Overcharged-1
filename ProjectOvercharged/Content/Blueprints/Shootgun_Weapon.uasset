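; Shotgun weapon Blueprint with limited ammo, a timed reload and randomized hitscan spread.
; Fire, while ammo remains, decrements the count, plays an animation unless the player is reloading, then runs a single randomly offset trace from the first-person camera.
; A second trace runs from the weapon's Scene component to that impact point; both draw debug lines and neither applies damage.
; Reload plays an animation, waits, then refills ammo to maximum.
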(event EventBeginPlay
  (|CallParentFunction) ; This node is disabled and will not be called.\nDrag off pins to build functionality.
)

(event Collision|EventActorBeginOverlap
  (params (OtherActor :type Actor%20Object%20Reference))
  (|CallParentFunction OtherActor) ; This node is disabled and will not be called.\nDrag off pins to build functionality.
)

(event EventTick
  (params (DeltaSeconds :type Float%20%28single-precision%29))
  (|CallParentFunction DeltaSeconds) ; This node is disabled and will not be called.\nDrag off pins to build functionality.
)

(event EventFire
  (if (> (Variables|Default|GetAmmoCount) 0)
    (CallFunction|AmmoCheck)
    (CallFunction|LineTrace)))

(event EventReload
  (Components|Animation|PlayAnimation (Variables|Default|GetSkeletalMesh) 0 false)
  (Utilities|FlowControl|Delay (Variables|Default|GetReloadTime))
  (Variables|Default|SetAmmoCount (Variables|Default|GetMaxAmmo)))

(fn ConstructionScript
  (|CallParentFunction)
  (Variables|Default|SetMaxAmmo 7)
  (Variables|Default|SetAmmoCount 7)
  (Variables|Default|SetReloadTime 2.0)
  (Variables|Default|SetBulletSpray 5e+02))

(fn AmmoCheck
  (Math|Integer|DecrementInt (Variables|Default|GetAmmoCount)
    (:%20%20
      (if (not (Variables|/Game/FirstPersonBP/Blueprints/FirstPersonCharacter.FirstPersonCharacter_C|GetIsReload (.AsFirst%20Person%20Character (Utilities|Casting|CastToFirstPersonCharacter (Game|GetPlayerCharacter 0)))))
        (Components|Animation|PlayAnimation (Variables|Default|GetSkeletalMesh) 0 false)))))

(fn LineTrace
  (bind _returnvalue (Game|GetPlayerCharacter 0))
  (bind _bulletspray (Variables|Default|GetBulletSpray))
  (bind _returnvalue_2 (* _bulletspray -1.0))
  (bind _asfirst_person_character (Utilities|Casting|CastToFirstPersonCharacter _returnvalue))
  (bind _firstpersoncamera (Variables|/Game/FirstPersonBP/Blueprints/FirstPersonCharacter.FirstPersonCharacter_C|GetFirstPersonCamera _asfirst_person_character))
  (bind _returnvalue_3 (Transformation|GetWorldLocation _firstpersoncamera))
  (bind _outhit (Collision|LineTraceByChannel _returnvalue_3 (+ (+ _returnvalue_3 (* (Math|Vector|GetForwardVector _firstpersoncamera) 2e+04)) (Math|Vector|MakeVector (Math|Random|RandomFloatinRange _returnvalue_2 _bulletspray) (Math|Random|RandomFloatinRange _returnvalue_2 _bulletspray) (Math|Random|RandomFloatinRange _returnvalue_2 _bulletspray))) "TraceTypeQuery1" false 0 "ForDuration"))
  (Collision|LineTraceByChannel (Transformation|GetWorldLocation (Variables|Default|GetScene)) (.ImpactPoint (Collision|BreakHitResult _outhit)) "TraceTypeQuery1" false 0 "ForDuration" true "(R=0.000000,G=1.000000,B=0.172742,A=1.000000)"))